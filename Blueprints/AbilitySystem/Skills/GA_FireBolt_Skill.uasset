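; Fire Bolt gameplay ability that casts homing fire projectiles from the caster's weapon socket.
; It targets the player's auto-target lock if valid, otherwise the location and actor under the mouse, and turns the avatar toward that point.
; A cast montage plays, its FireBolt gameplay event triggers the projectile spawn, and montage completion, blend out or interruption ends the ability.
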(event Ability|EventActivateAbility
  (Development|PrintString (Utilities|String|ToString(Integer) (Utilities|Map|Length (Variables|Default|GetTalentsTree))) true true "(R=1.000000,G=0.072917,B=0.072917,A=1.000000)" 3.0)
  ;[1 1 1] The ability will be prevented to be activated if it dont have the ressources availables
  (Ability|CommitAbility)
  (Class|AuraGameplayAbility|StoreOwnerVariables)
  (Utilities|IsValid (Variables|/Script/Aura.AuraPlayerController|GetTargetLock (Variables|Default|GetOwnerPlayerController))
    (:Is%20Valid
      ;[1 1 1] Instead of Store Mouse Data, we use the Target from AutoTarget
      (Variables|Default|SetMouseHitActor (Variables|/Script/Aura.AuraPlayerController|GetTargetLock (Variables|Default|GetOwnerPlayerController)))
      (Variables|Default|SetProjectileTargetLocation (Transformation|GetActorLocation (Variables|/Script/Aura.AuraPlayerController|GetTargetLock (Variables|Default|GetOwnerPlayerController)))))
    (:Is%20Not%20Valid
      (bind _datahandle (|TargetDataUnderMouse)
        (:ValidData
          (Variables|Default|SetProjectileTargetLocation (.Location (Collision|BreakHitResult (Ability|TargetData|GetHitResultfromTargetData _datahandle))))
          (Variables|Default|SetMouseHitActor (.HitActor (Collision|BreakHitResult (Ability|TargetData|GetHitResultfromTargetData _datahandle))))))))
  (Class|CombatInterface|UpdateFacingTarget(Message) (Ability|GetAvatarActorfromActorInfo) (Variables|Default|GetProjectileTargetLocation))
  (|PlayMontageandWaitProxy "None" "/Game/Assets/Characters/Aura/Animations/Abilities/AM_Cast_FireBolt.AM_Cast_FireBolt" 1.0 "None" false 1.0 0.0 false
    (:then
      (Ability|Tasks|WaitGameplayEvent "(TagName=\"Event.Montage.FireBolt\")" 0
        (:then
          (Class|FireboltSkill|SpawnProjectiles (Variables|Default|GetProjectileTargetLocation) (GameplayTags|MakeLiteralGameplayTag "(TagName=\"CombatSocket.Weapon\")") true 1e+01 (Variables|Default|GetMouseHitActor)))))
    (:OnCompleted
      (Ability|EndAbility :!label _label))
    (:OnBlendOut
      (goto _label))
    (:OnInterrupted
      (goto _label))
    (:OnCancelled
      (goto _label))))