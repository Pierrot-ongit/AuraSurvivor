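; Gameplay ability that casts chain lightning at the locked target or cursor, jumping between targets.
; On the montage's Electrocute event it hits the first target, then repeatedly finds the next from the last, up to a maximum count.
; CombatInterface targets take SetByCaller lightning damage; each link adds a GameplayCue attached to the weapon or previous target.
; Cue parameters are stored per actor to remove cues after a post-montage delay.
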(event Ability|EventActivateAbility
  ;[1 1 1] The ability will be prevented to be activated if it dont have the ressources availables
  (Ability|CommitAbility)
  (Class|AuraGameplayAbility|StoreOwnerVariables)
  (Utilities|IsValid (Variables|/Script/Aura.AuraPlayerController|GetTargetLock (Variables|Default|GetOwnerPlayerController))
    (:Is%20Valid
      ;[1 1 1] Instead of Store Mouse Data, we use the Target from AutoTarget
      (Variables|Default|SetMouseHitActor (Variables|/Script/Aura.AuraPlayerController|GetTargetLock (Variables|Default|GetOwnerPlayerController)))
      (Variables|Default|SetMouseHitLocation (Transformation|GetActorLocation (Variables|/Script/Aura.AuraPlayerController|GetTargetLock (Variables|Default|GetOwnerPlayerController)))))
    (:Is%20Not%20Valid
      ;[1 0.276 0.276] Store Mouse Data Variables
      (bind _datahandle (|TargetDataUnderMouse)
        (:ValidData
          (Class|SkillBeam|StoreMouseDataInfo (Ability|TargetData|GetHitResultfromTargetData _datahandle))))))
  (Class|CombatInterface|UpdateFacingTarget(Message) (Ability|GetAvatarActorfromActorInfo) (Variables|Default|GetMouseHitLocation))
  (|PlayMontageandWaitProxy "None" "/Game/Assets/Characters/Aura/Animations/Abilities/AM_Cast_Long.AM_Cast_Long" 1.0 "None" false 1.0 0.0 false
    (:then
      (Ability|Tasks|WaitGameplayEvent "(TagName=\"Event.Montage.Electrocute\")" 0 true
        (:EventReceived
          (Class|SkillBeam|TraceFirstTarget (Variables|Default|GetMouseHitLocation))
          (CallFunction|SpawnLightningChain (Variables|Default|GetMouseHitActor) (Variables|Default|GetMouseHitLocation) true)
          (Utilities|IsValid (Variables|Default|GetLastTarget)
            (:Is%20Valid
              (bind _returnvalue (Class|SkillBeam|GetMaxNumChainTargets))
              (for _index (range 2 _returnvalue)
                (bind _returnvalue_2 (Class|SkillBeam|FindNextTarget (Transformation|GetActorLocation (Variables|Default|GetLastTarget))))
                (Utilities|IsValid _returnvalue_2
                  (:Is%20Valid
                    (CallFunction|SpawnLightningChain _returnvalue_2 (Transformation|GetActorLocation (Variables|Default|GetLastTarget)) false)))))))))
    (:OnCompleted
      (Utilities|FlowControl|Delay (Variables|Default|GetDelayBeforeEnd) :!label _label)
      (CallFunction|PreparetoEndAbility)
      (Ability|EndAbility))
    (:OnBlendOut
      (goto _label))
    (:OnInterrupted
      (goto _label))
    (:OnCancelled
      (goto _label))))

(fn ApplySingleDamage
  (params (Actor :type Actor%20Object%20Reference))
  (LocalVariables|SetDamagedTarget Actor)
  (bind _output_get (LocalVariables|SetASC (Ability|GetAbilitySystemComponentfromActorInfo)))
  (Utilities|IsValid _output_get
    (:Is%20Valid
      (bind _returnvalue (Ability|GameplayEffect|AssignTagSetbyCallerMagnitude (GameplayEffects|MakeOutgoingSpec (LocalVariables|GetASC) (Variables|Default|GetDamageEffectClass) (Math|Conversions|ToFloat(Integer) (Ability|GetAbilityLevel)) (GameplayEffects|MakeEffectContext (LocalVariables|GetASC))) "(TagName=\"Damage.Lightning\")" (Class|AuraDamageGameplayAbility|GetDamageatLevel)))
      (Utilities|IsValid (Ability|GetAbilitySystemComponent (LocalVariables|GetDamagedTarget))
        (:Is%20Valid
          (GameplayEffects|ApplyGameplayEffectSpecToSelf (Ability|GetAbilitySystemComponent (LocalVariables|GetDamagedTarget)) _returnvalue))))))

(fn SpawnLightningChain
  (params (TargetActor :type Actor%20Object%20Reference) (TargetLocation :type Vector) (ChainBegin :type Boolean))
  (LocalVariables|SetTarget TargetActor)
  (LocalVariables|SetCueLocation TargetLocation)
  (if ChainBegin
    (bind _returnvalue (Class|CombatInterface|GetWeapon(Message) (Variables|Default|GetOwnerCharacter)))
    (LocalVariables|SetAttachComponent _returnvalue)
    (else
      (LocalVariables|SetAttachComponent (Variables|/Script/Engine.Actor|GetRootComponent (Variables|Default|GetLastTarget)))))
  (LocalVariables|SetCueParams (Ability|GameplayCue|MakeGameplayCueParameters :Location (LocalVariables|GetCueLocation) :SourceObject (LocalVariables|GetTarget) :TargetAttachComponent (LocalVariables|GetAttachComponent)))
  ;[1 1 1] Is Target an Enemy
  (if (Utilities|DoesObjectImplementInterface (LocalVariables|GetTarget) "/Script/Aura.CombatInterface")
    (bind _output_get (LocalVariables|SetCueTarget (LocalVariables|GetTarget)))
    (CallFunction|ApplySingleDamage _output_get)
    (else
      (LocalVariables|SetCueTarget (Variables|Default|GetOwnerCharacter))))
  (GameplayCue|AddGameplayCueOnActor(Looping) (LocalVariables|GetCueTarget) "(TagName=\"GameplayCue.LightningChain\")" (LocalVariables|GetCueParams))
  (Utilities|Array|AddUnique (Variables|Default|GetTargetsChained) (LocalVariables|GetCueTarget))
  (Utilities|Map|Add (Variables|Default|GetTargetsChainedCueParams) (LocalVariables|GetCueTarget) (LocalVariables|GetCueParams))
  (Variables|Default|SetLastTarget (LocalVariables|GetCueTarget)))

(fn RemoveCuefromActor
  (params (Actor :type Actor%20Object%20Reference%20%28by%20ref%29))
  (bind _targetschainedcueparams (Variables|Default|GetTargetsChainedCueParams))
  (bind (_value _returnvalue) (Utilities|Map|Find _targetschainedcueparams Actor))
  (if _returnvalue
    (GameplayCue|RemoveGameplayCueOnActor(Looping) Actor "(TagName=\"GameplayCue.LightningChain\")" _value)))

(fn PreparetoEndAbility
  (for _array_element (Variables|Default|GetTargetsChained)
    (CallFunction|RemoveCuefromActor _array_element))
  (Variables|Default|SetMouseHitActor 0)
  (Utilities|Array|Clear (Variables|Default|GetTargetsChained))
  (Utilities|Map|Clear (Variables|Default|GetTargetsChainedCueParams)))